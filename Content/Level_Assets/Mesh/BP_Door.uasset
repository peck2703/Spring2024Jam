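; BP_Door is an interactable hinged door that swings open or closed each time it is interacted with.
; Interact calls OpenDoor, where a FlipFlop plays or reverses a timeline that lerps the Door's relative yaw, and plays a creak sound at the actor's location.
; A Box overlap shows an "E" prompt on the first-person character's HUD and clears it on exit.
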(event OnComponentBeginOverlap(Box)
  (params (OverlappedComponent :type Primitive%20Component%20Object%20Reference) (OtherActor :type Actor%20Object%20Reference) (OtherComp :type Primitive%20Component%20Object%20Reference) (OtherBodyIndex :type Integer) (bFromSweep :type Boolean) (SweepResult :type Hit%20Result%20Structure%20%28by%20ref%29))
  (bind _asbp_first_person_character (Utilities|Casting|CastToBP_FirstPersonCharacter OtherActor))
  (Default|SetInteractText (Variables|/Game/Blueprints/BP_FirstPersonCharacter.BP_FirstPersonCharacter_C|GetMainHUD_Ref _asbp_first_person_character) "E"))

(event OnComponentEndOverlap(Box)
  (params (OverlappedComponent :type Primitive%20Component%20Object%20Reference) (OtherActor :type Actor%20Object%20Reference) (OtherComp :type Primitive%20Component%20Object%20Reference) (OtherBodyIndex :type Integer))
  (bind _asbp_first_person_character (Utilities|Casting|CastToBP_FirstPersonCharacter OtherActor))
  (Default|SetInteractText (Variables|/Game/Blueprints/BP_FirstPersonCharacter.BP_FirstPersonCharacter_C|GetMainHUD_Ref _asbp_first_person_character)))

(event Custom|Open%20Door
  (Utilities|FlowControl|FlipFlop
    (:A
      (bind _doorfloat (Timeline|Open%20Door%20Lag Play)
        (:Update
          (Transformation|SetRelativeRotation (Variables|Default|GetDoor) (Math|Rotator|MakeRotator 0.0 0.0 (Math|Float|Lerp 0.0 -9e+01 _doorfloat)) false false))))
    (:B
      (Timeline|Open%20Door%20Lag Reverse))))

(event EventBeginPlay)

(event Collision|EventActorBeginOverlap
  (params (OtherActor :type Actor%20Object%20Reference)))

(event EventTick
  (params (DeltaSeconds :type Float%20%28single-precision%29)))

(event EventInteract
  (CallFunction|OpenDoor)
  (Audio|PlaySoundatLocation "/Game/Audio/SFX/Environment/CreekyDoorOpen.CreekyDoorOpen" (Transformation|GetActorLocation) "0, 0, 0" 1.0 1.0 0.0 0 0 0 0))

(fn ConstructionScript)