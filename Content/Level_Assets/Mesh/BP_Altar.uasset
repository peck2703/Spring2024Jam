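; BP_Altar is an interactable altar that displays the Mercury, Salt and Sulphur items the player holds.
; Interact calls CheckStones, which reads the three possession flags from the first BP_FirstPersonCharacter found in the level.
; For each set flag, a DoOnce-gated branch spawns the matching item actor at its named socket on the AltarLP mesh.
; The player's flags are left unchanged.
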(event Custom|CheckStones
  (bind _outactors (Actor|GetAllActorsOfClass "/Game/Blueprints/BP_FirstPersonCharacter.BP_FirstPersonCharacter_C"))
  (Utilities|FlowControl|Sequence
    (:then_0
      (if (Variables|/Game/Blueprints/BP_FirstPersonCharacter.BP_FirstPersonCharacter_C|GetHasMercury (Utilities|Array|Get(acopy) _outactors))
        (Utilities|FlowControl|DoOnce false
          (:Completed
            (Game|SpawnActorfromClass "/Game/Level_Assets/Mesh/BP_Mercury_Item.BP_Mercury_Item_C" (CallFunction|GetSocket "Mercury" "RTS_World") "Undefined" "MultiplyWithRoot" 0 0)))))
    (:then_1
      (if (Variables|/Game/Blueprints/BP_FirstPersonCharacter.BP_FirstPersonCharacter_C|GetHasSalt (Utilities|Array|Get(acopy) _outactors))
        (Utilities|FlowControl|DoOnce false
          (:Completed
            (Game|SpawnActorfromClass "/Game/Level_Assets/Mesh/BP_Salt_Item.BP_Salt_Item_C" (CallFunction|GetSocket "Salt" "RTS_World") "Undefined" "MultiplyWithRoot" 0 0)))))
    (:then_2
      (if (Variables|/Game/Blueprints/BP_FirstPersonCharacter.BP_FirstPersonCharacter_C|GetHasSulphur (Utilities|Array|Get(acopy) _outactors))
        (Utilities|FlowControl|DoOnce false
          (:Completed
            (Game|SpawnActorfromClass "/Game/Level_Assets/Mesh/BP_Sulphur_Item.BP_Sulphur_Item_C" (CallFunction|GetSocket "Sulphur" "RTS_World") "Undefined" "MultiplyWithRoot" 0 0)))))))

(event EventBeginPlay)

(event Collision|EventActorBeginOverlap
  (params (OtherActor :type Actor%20Object%20Reference)))

(event EventTick
  (params (DeltaSeconds :type Float%20%28single-precision%29)))

(event EventInteract
  (CallFunction|CheckStones))

(fn ConstructionScript)

(fn GetSocket
  (params (InSocketName :type Name) (TransformSpace :type ERelativeTransformSpace%20Enum :default "RTS_World"))
  (return (Transformation|GetSocketTransform (Variables|Default|GetAltar_LP) InSocketName TransformSpace)))