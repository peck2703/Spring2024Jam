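; BP_Mercury_Pillar_Blueprint is a level pillar that slides to an end position once it has been triggered twice.
; Each GetCounter call increments a counter and calls Lower, which at two or more passes a DoOnce, plays a sliding-stone sound and starts a timeline.
; The timeline moves the actor toward EndPos, lerping from its current location on every update rather than from a stored start.
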(event Custom|GetCounter
  (Variables|Default|SetCounter (+ (Variables|Default|GetCounter) 1))
  (CallFunction|Lower))

(event Custom|Lower
  (if (>= (Variables|Default|GetCounter) 2)
    (Utilities|FlowControl|DoOnce false
      (:Completed
        (Audio|PlaySoundatLocation "/Game/Audio/SFX/Environment/Sliding_Stone_Loop.Sliding_Stone_Loop" (Transformation|GetActorLocation) "0, 0, 0" 1.0 1.0 0.0 0 0 0 0)
        (bind _alpha (Timeline|LowerTime Play)
          (:Update
            (Transformation|SetActorLocation (Math|Vector|Lerp(Vector) (Transformation|GetActorLocation) (Variables|Default|GetEndPos) _alpha) false false)))))))

(event EventBeginPlay)

(event Collision|EventActorBeginOverlap
  (params (OtherActor :type Actor%20Object%20Reference)))

(event EventTick
  (params (DeltaSeconds :type Float%20%28single-precision%29)))

(fn ConstructionScript)