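; BP_Mercury_Item is a collectible Mercury pickup that spins on a tilted axis in the level.
; Tick plays a timeline that drives the root's yaw through its rotation with a fixed roll.
; Interact calls AddToPlayer, which sets HasMercury on the first BP_FirstPersonCharacter found in the world and destroys the item, then plays a 2D pickup chime.
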(event Custom|AddToPlayer
  (bind _outactors (Actor|GetAllActorsOfClass "/Game/Blueprints/BP_FirstPersonCharacter.BP_FirstPersonCharacter_C"))
  (Variables|/Game/Blueprints/BP_FirstPersonCharacter.BP_FirstPersonCharacter_C|SetHasMercury (Utilities|Array|Get(acopy) _outactors) true)
  (Actor|DestroyActor))

(event EventBeginPlay)

(event Collision|EventActorBeginOverlap
  (params (OtherActor :type Actor%20Object%20Reference)))

(event EventTick
  (params (DeltaSeconds :type Float%20%28single-precision%29))
  (bind _defaultsceneroot (Variables|Default|GetDefaultSceneRoot))
  (bind _rotation (Timeline|Timeline_1 Play)
    (:Update
      (Transformation|SetRelativeLocationAndRotation _defaultsceneroot (Variables|/Script/Engine.SceneComponent|GetRelativeLocation _defaultsceneroot) (Math|Rotator|MakeRotator -2e+01 0.0 (* _rotation 3.6e+02)) false false))))

(event EventInteract
  (CallFunction|AddtoPlayer)
  (Audio|PlaySound2D "/Game/Audio/SFX/General/Pickup_Chime.Pickup_Chime" 1.0 1.0 0.0 0 0))

(fn ConstructionScript)