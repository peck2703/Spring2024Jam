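; BP_LightningAttack is a lightning effect actor that arcs to nearby surfaces and activates electrical objects it touches.
; On a cooldown checked each tick, it line-traces in a random direction between two radii and spawns an attached Niagara arc toward any blocking hit.
; Separately, actors overlapping its Collision component that implement BPI_Electric receive an activate message and trigger a chime.
; A lightning sound plays at its sphere's location on BeginPlay.
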(event OnComponentBeginOverlap(Collision)
  (params (OverlappedComponent :type Primitive%20Component%20Object%20Reference) (OtherActor :type Actor%20Object%20Reference) (OtherComp :type Primitive%20Component%20Object%20Reference) (OtherBodyIndex :type Integer) (bFromSweep :type Boolean) (SweepResult :type Hit%20Result%20Structure%20%28by%20ref%29))
  ;[0 0 0] If object "hit" has interface for Electricity, then activate command (in that actors blueprint)
  (if (Utilities|DoesObjectImplementInterface OtherActor "/Game/Blueprints/Interaction/Interface/BPI_Electric.BPI_Electric_C")
    (bind _output_get (Variables|Default|SetHit%20Actor OtherActor))
    (Class|BPIElectric|Activate(Message) _output_get)
    (Audio|PlaySound2D "/Game/Audio/SFX/General/Correct_Chime.Correct_Chime" 0.5 1.0 0.0 0 0)))

(event EventBeginPlay
  (Audio|PlaySoundatLocation "/Game/Audio/SFX/Environment/Elements/Lightning_Loop.Lightning_Loop" (Transformation|GetWorldLocation (Variables|Default|GetSphere)) "0, 0, 0" 1.0 1.0 0.0 0 0 0 0)
  (Variables|Default|SetLastSound 0.0))

(event EventTick
  (params (DeltaSeconds :type Float%20%28single-precision%29))
  (CallFunction|UpdateTraces))

(fn ConstructionScript)

(fn UpdateTraces
  (bind _returnvalue (Transformation|GetActorLocation))
  (if (>= (- (Utilities|Time|GetTimeSeconds) (Variables|Default|GetLastTrace)) (Variables|Default|GetTraceCooldown))
    ;[1 1 1] Lighteningbolt line trace
    (Variables|Default|SetForwardDirection (Math|Random|RandomUnitVector))
    (bind _outhit (Collision|LineTraceByChannel (+ _returnvalue (* (Variables|Default|GetForwardDirection) (Variables|Default|GetMinRadius))) (+ _returnvalue (* (Variables|Default|GetForwardDirection) (Variables|Default|GetMaxRadius))) "TraceTypeQuery1" false 0 "None" true "(R=1.000000,G=0.000000,B=0.000000,A=1.000000)" "(R=0.000000,G=1.000000,B=0.000000,A=1.000000)" (Variables|Default|GetTraceCooldown)))
    (Variables|Default|SetLastTrace (Utilities|Time|GetTimeSeconds))
    ;[1 1 1] Spawn NiagaraSystem
    (if (.bBlockingHit (Collision|BreakHitResult _outhit))
      (bind _returnvalue_2 (Niagara|SpawnSystemAttached "/Game/Level_Assets/Materials/FX/Lightning/FX_LightingArcs.FX_LightingArcs" (Variables|Default|GetDefaultSceneRoot) "None" "0, 0, 0" "0, 0, 0" "KeepRelativeOffset" false))
      (Niagara|SetNiagaraVariable(Vector3) _returnvalue_2 "BeamStartPoint" (* (Variables|Default|GetForwardDirection) (Variables|Default|GetMinRadius)))
      (Niagara|SetNiagaraVariable(Vector3) _returnvalue_2 "BeamEndPoint" (+ (.ImpactPoint (Collision|BreakHitResult _outhit)) (* (.ImpactNormal (Collision|BreakHitResult _outhit)) (Variables|Default|GetImpactOffest))))
      (Niagara|SetNiagaraVariable(Vector3) _returnvalue_2 "ImpactNormal" (.ImpactNormal (Collision|BreakHitResult _outhit))))))