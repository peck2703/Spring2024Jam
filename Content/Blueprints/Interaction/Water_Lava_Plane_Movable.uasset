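; Movable water or lava hazard plane with a configurable surface material, applied in the construction script.
; A one-shot Lower event runs a timeline that lerps the actor from its current location toward EndPos.
; Its KillBox reloads the current level two seconds after the first-person character enters and destroys mushroom and clay element actors.
; Steam interact actors overlapping the plane receive a BeforeDeath call.
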(event OnComponentBeginOverlap(KillBox)
  (params (OverlappedComponent :type Primitive%20Component%20Object%20Reference) (OtherActor :type Actor%20Object%20Reference) (OtherComp :type Primitive%20Component%20Object%20Reference) (OtherBodyIndex :type Integer) (bFromSweep :type Boolean) (SweepResult :type Hit%20Result%20Structure%20%28by%20ref%29))
  (Utilities|Casting|CastToBP_FirstPersonCharacter OtherActor
    (:then
      (bind _returnvalue (Game|GetCurrentLevelName true))
      (Utilities|FlowControl|Delay 2.0)
      (Game|OpenLevel(byName) (Utilities|String|StringToName _returnvalue)))
    (:CastFailed
      (bind _asbp_element_mushrooms (Utilities|Casting|CastToBP_Element_Mushrooms OtherActor)
        (:then
          (Actor|DestroyActor _asbp_element_mushrooms))
        (:CastFailed
          (bind _asbp_element_clay (Utilities|Casting|CastToBP_Element_Clay OtherActor))
          (Actor|DestroyActor _asbp_element_clay))))))

(event Custom|Lower
  (Utilities|FlowControl|DoOnce false
    (:Completed
      (bind _alpha (Timeline|Lower_Timeline Play)
        (:Update
          (Transformation|SetActorLocation (Math|Vector|Lerp(Vector) (Transformation|GetActorLocation) (Variables|Default|GetEndPos) _alpha) false false))))))

(event EventBeginPlay)

(event Collision|EventActorBeginOverlap
  (params (OtherActor :type Actor%20Object%20Reference))
  (bind _asbp_steam_interact_m (Utilities|Casting|CastToBP_Steam_Interact_M OtherActor))
  (Default|BeforeDeath _asbp_steam_interact_m))

(event EventTick
  (params (DeltaSeconds :type Float%20%28single-precision%29)))

(fn ConstructionScript
  (Rendering|Material|SetMaterial (Variables|Default|GetWater) 0 (Variables|Default|GetWater-Lava_Mat)))