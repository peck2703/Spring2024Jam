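; Interaction component that line traces from the player camera to find the object in view.
; StartTrace runs a Visibility trace with configurable length and debug drawing, stores the hit actor in HitObject, and prints its name for testing.
; LineTraceLocations derives the start and end points from the camera's location and forward vector.
; The planned elemental spell step at the end of the trace is not yet implemented.
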(event Custom|StartTrace
  (params (VectorLength :type Float%20%28double-precision%29) (DrawDebugType :type EDrawDebugTrace%20Enum :default "None"))
  (bind (_start _end) (CallFunction|LineTraceLocations VectorLength))
  ;[0 0 0] Full Line Trace with Debug. Need to add elemental spell to end of logic.
  (bind _outhit (Collision|LineTraceByChannel _start _end "TraceTypeQuery1" false 0 DrawDebugType false))
  (bind _output_get (Variables|Default|SetHitObject (.HitActor (Collision|BreakHitResult _outhit))))
  ;;[1 1 1] Testing
  (Development|PrintString (Utilities|GetDisplayName _output_get)))

(fn LineTraceLocations
  (params (Length :type Float%20%28double-precision%29))
  (bind _player_ref (Variables|Default|GetPlayer_Ref))
  (bind _camera (Variables|/Game/Blueprints/BP_FirstPersonCharacter.BP_FirstPersonCharacter_C|GetCamera _player_ref))
  (bind _returnvalue (Transformation|GetWorldLocation _camera))
  (return _returnvalue (+ _returnvalue (* (Math|Vector|GetForwardVector _camera) Length))))