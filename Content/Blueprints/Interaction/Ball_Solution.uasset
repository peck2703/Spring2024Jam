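; Ball_Solution is a puzzle target that checks whether a BP_Steam_Interact_M actor entering its Sphere collider carries the matching material.
; On overlap, it compares the first material slot of that actor's static mesh against MaterialToMatch.
; A match calls GetCounter on the first BP_Mercury_Pillar_Blueprint found in the level.
; A mismatch calls BeforeDeath on the overlapping actor.
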(event OnComponentBeginOverlap(Sphere)
  (params (OverlappedComponent :type Primitive%20Component%20Object%20Reference) (OtherActor :type Actor%20Object%20Reference) (OtherComp :type Primitive%20Component%20Object%20Reference) (OtherBodyIndex :type Integer) (bFromSweep :type Boolean) (SweepResult :type Hit%20Result%20Structure%20%28by%20ref%29))
  (bind _asbp_steam_interact_m (Utilities|Casting|CastToBP_Steam_Interact_M OtherActor))
  (bind _output_get (Variables|Default|SetCorrectSphereCollider (== (Rendering|Material|GetMaterial (Variables|/Game/Blueprints/Interaction/BP_Steam_Interact_M.BP_Steam_Interact_M_C|GetStaticMesh _asbp_steam_interact_m) 0) (Variables|Default|GetMaterialToMatch))))
  (if _output_get
    (bind _outactors (Actor|GetAllActorsOfClass "/Game/Level_Assets/Mesh/BP_Mercury_Pillar_Blueprint.BP_Mercury_Pillar_Blueprint_C"))
    (Default|GetCounter (Utilities|Array|Get(acopy) _outactors))
    (else
      (Default|BeforeDeath _asbp_steam_interact_m))))

(event EventBeginPlay)

(event Collision|EventActorBeginOverlap
  (params (OtherActor :type Actor%20Object%20Reference)))

(event EventTick
  (params (DeltaSeconds :type Float%20%28single-precision%29)))

(fn ConstructionScript)