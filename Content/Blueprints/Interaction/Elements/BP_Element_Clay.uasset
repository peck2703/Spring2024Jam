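; Clay interaction element: a scalable cube that is carried in front of the player and can be dropped onto surfaces below.
; A looping timer keeps it at the player's SpawnComponent, with a scale-based offset on X only, while Resize uniformly scales it within limits from scroll input.
; DropClay stops the timer, box-traces (zero half-size) along ZAmount, and on a hit the Landing timeline sets collision to Block and lerps Z to rest.
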(event Custom|Begin
  (bind _player_ref (Variables|Default|GetPlayer_Ref))
  (bind _spawncomponent (Variables|/Game/Blueprints/BP_FirstPersonCharacter.BP_FirstPersonCharacter_C|GetSpawnComponent _player_ref))
  (bind _returnvalue (Transformation|GetWorldLocation _spawncomponent))
  (Transformation|SetActorLocation (Math|Vector|MakeVector (+ (.x _returnvalue) (CallFunction|AddForwardMovement)) (.y _returnvalue) (.z _returnvalue)) false false))

(event Custom|Resize
  (params (Value :type Float%20%28double-precision%29))
  (bind _scale (CallFunction|GetCubeScale))
  (bind _returnvalue (CallFunction|ChangeScale Value _scale))
  ;[0 0 0] Negative scroll, must be above min scale
  (if (< Value 0.0)
    (if (> (CallFunction|GetCubeScale) (Variables|Default|GetMinScale))
      (Transformation|SetWorldScale3D (Variables|Default|GetCube) _returnvalue))
    (elif (< _scale (Variables|Default|GetMaxScale))
      (Transformation|SetWorldScale3D (Variables|Default|GetCube) _returnvalue))))

(event Custom|DropClay
  (bind _returnvalue (Transformation|GetActorLocation))
  (bind _cube (Variables|Default|GetCube))
  (bind _returnvalue_2 (Transformation|GetWorldLocation _cube))
  (Utilities|Time|ClearandInvalidateTimerbyHandle (Variables|Default|GetMovementTimer))
  (bind (_outhit _returnvalue_3) (Collision|BoxTraceByChannel _returnvalue_2 (+ _returnvalue_2 (Variables|Default|GetZAmount)) (CallFunction|HalfBoxShape) "0, 0, 0" "TraceTypeQuery1" false 0 "None"))
  (if _returnvalue_3
    (bind _alpha (Timeline|Landing Play)
      (:Update
        (Collision|SetCollisionResponsetoAllChannels (Variables|Default|GetCube) "ECR_Block")
        (Transformation|SetActorLocation (Math|Vector|MakeVector (.x _returnvalue) (.y _returnvalue) (Math|Float|Lerp (.z _returnvalue) (.z (- (.ImpactPoint (Collision|BreakHitResult _outhit)) (Math|Vector|MakeVector 0.0 0.0 (.z (Transformation|GetWorldScale (Variables|Default|GetCube)))))) _alpha)) false false)))))

(event EventBeginPlay
  (|CallParentFunction)
  (bind _returnvalue (Utilities|Time|SetTimerbyEvent (delegate Custom|Begin) 0.03125 true))
  (Variables|Default|SetMovementTimer _returnvalue))

(fn ConstructionScript
  (|CallParentFunction)
  (Variables|Default|SetScale (Transformation|GetWorldScale (Variables|Default|GetCube))))

(fn GetCubeScale
  (return (.Z (Math|Vector|BreakVector (Transformation|GetWorldScale (Variables|Default|GetCube))))))

(fn ChangeScale
  (params (Scroll :type Float%20%28double-precision%29) (WorldScale :type Float%20%28double-precision%29))
  (bind _rateofgrowth (Variables|Default|GetRateOfGrowth))
  (bind _returnvalue (* Scroll _rateofgrowth))
  (bind _returnvalue_2 (+ _returnvalue WorldScale))
  (return (Math|Vector|MakeVector _returnvalue_2 _returnvalue_2 _returnvalue_2)))

(fn ChangeinDistance
  (params (ScaleUp? :type Boolean))
  (bind _distancetomove (Variables|Default|GetDistanceToMove))
  (bind _cube (Variables|Default|GetCube))
  (bind _relativelocation (Variables|/Script/Engine.SceneComponent|GetRelativeLocation _cube))
  (if ScaleUp?
    (return (+ _relativelocation _distancetomove))
    (else
      (return (- _relativelocation _distancetomove)))))

(fn IsFalling
  (bind _cube (Variables|Default|GetCube))
  (bind _returnvalue (Transformation|GetComponentVelocity _cube))
  (return (or (> (.z _returnvalue) 0.0) (< (.z _returnvalue) 0.0))))

(fn HalfBoxShape
  (return (/ (* "" (Transformation|GetWorldScale (Variables|Default|GetCube))) 2.0)))

(fn AddForwardMovement
  (return (* (.x (Transformation|GetActorForwardVector)) (.x (Transformation|GetWorldScale (Variables|Default|GetCube))) (Variables|Default|GetForwardVectorMultiplier))))