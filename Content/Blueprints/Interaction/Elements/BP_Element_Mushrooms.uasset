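; Mushroom element actor that the player carries, drops and grows into a bounce pad.
; After BeginPlay a looping timer keeps it snapped to the player's spawn component until DropMushroom clears the timer.
; Dropping line-traces to a surface, then timelines lerp it down and scale it up with a slight rise.
; Overlapping its box launches the first-person character by UpwardsVelocity with a bounce sound.
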(event OnComponentHit(Box)
  (params (HitComponent :type Primitive%20Component%20Object%20Reference) (OtherActor :type Actor%20Object%20Reference) (OtherComp :type Primitive%20Component%20Object%20Reference) (NormalImpulse :type Vector :default "0, 0, 0") (Hit :type Hit%20Result%20Structure%20%28by%20ref%29)))

(event OnComponentBeginOverlap(Box)
  (params (OverlappedComponent :type Primitive%20Component%20Object%20Reference) (OtherActor :type Actor%20Object%20Reference) (OtherComp :type Primitive%20Component%20Object%20Reference) (OtherBodyIndex :type Integer) (bFromSweep :type Boolean) (SweepResult :type Hit%20Result%20Structure%20%28by%20ref%29))
  (bind _asbp_first_person_character (Utilities|Casting|CastToBP_FirstPersonCharacter OtherActor))
  (Character|LaunchCharacter _asbp_first_person_character (Variables|Default|GetUpwardsVelocity) false false)
  (Audio|PlaySoundatLocation "/Game/Audio/SFX/Environment/Mushroom_Bounce.Mushroom_Bounce" (Transformation|GetActorLocation) "0, 0, 0" 1.0 1.0 0.0 0 0 0 0))

(event Custom|DropMushroom
  (bind _returnvalue (Transformation|GetActorLocation))
  (bind _mushroom (Variables|Default|GetMushroom))
  (bind _returnvalue_2 (Transformation|GetWorldLocation _mushroom))
  (Utilities|Time|ClearandInvalidateTimerbyHandle (Variables|Default|GetMoveActorTimer))
  (bind (_outhit _returnvalue_3) (Collision|LineTraceByChannel _returnvalue_2 (+ _returnvalue_2 (Variables|Default|GetZAmount)) "TraceTypeQuery1" false 0 "None"))
  (if _returnvalue_3
    (bind _alpha (Timeline|Landing Play)
      (:Update
        (Collision|SetCollisionResponsetoAllChannels (Variables|Default|GetMushroom) "ECR_Block")
        (Transformation|SetActorLocation (Math|Vector|MakeVector (.x _returnvalue) (.y _returnvalue) (Math|Float|Lerp (.z _returnvalue) (.z (.Location (Collision|BreakHitResult _outhit))) _alpha)) false false))
      (:Finished
        (CallFunction|GrowMushroom)
        (Audio|PlaySoundatLocation "/Game/Audio/SFX/Environment/Elements/Mushroom_Grow.Mushroom_Grow" (Transformation|GetActorLocation) "0, 0, 0" 1.0 1.0 0.0 0 0 0 0)))))

(event Custom|Begin
  (Transformation|SetActorLocation (Transformation|GetWorldLocation (Variables|/Game/Blueprints/BP_FirstPersonCharacter.BP_FirstPersonCharacter_C|GetSpawnComponent (Variables|Default|GetPlayer_Ref))) false false))

(event Custom|GrowMushroom
  (bind _returnvalue (Transformation|GetActorLocation))
  (bind _alpha (Timeline|GrowScale Play)
    (:Update
      (Transformation|SetActorTransform (Math|Transform|MakeTransform (Math|Vector|Lerp(Vector) _returnvalue (+ _returnvalue (* (Transformation|GetActorScale3D) "0.000000,0.000000,0.020000")) _alpha) "0, 0, 0" (Math|Vector|Lerp(Vector) (Transformation|GetActorScale3D) (Variables|Default|GetNewScale) _alpha))))))

(event EventBeginPlay
  (|CallParentFunction)
  (bind _returnvalue (Utilities|Time|SetTimerbyEvent (delegate Custom|Begin) 0.03125 true))
  (Variables|Default|SetMoveActorTimer _returnvalue))

(fn ConstructionScript
  (|CallParentFunction))