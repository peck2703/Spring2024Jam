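; Steam element power that lets the player push steam-interactive objects along the camera's aim.
; SetVariables and Reset compute a trace from the player's SpawnComponent along camera forward, which BeginPower fires with persistent debug drawing.
; Hits implementing BPI_Steamable are cast to BP_Steam_Interact_M, given a force-scaled Direction, then sent InteractMessage.
; On BeginPlay, a valid emitter triggers a wind sound and is spawned deactivated.
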(event Custom|BeginPower
  (bind (_outhit _returnvalue) (Collision|LineTraceByChannel (Variables|Default|GetStart) (Variables|Default|GetEnd) "TraceTypeQuery1" false 0 "Persistent"))
  (if _returnvalue
    (bind _output_get (Variables|Default|SetHit%20Actor (.HitActor (Collision|BreakHitResult _outhit))))
    (if (Utilities|DoesObjectImplementInterface (.HitActor (Collision|BreakHitResult _outhit)) "/Game/Blueprints/Interaction/Interface/BPI_Steamable.BPI_Steamable_C")
      (Variables|/Game/Blueprints/Interaction/BP_Steam_Interact_M.BP_Steam_Interact_M_C|SetDirection (.AsBP%20Steam%20Interact%20M (Utilities|Casting|CastToBP_Steam_Interact_M _output_get)) (* (CallFunction|GetDirection) (Variables|Default|GetForceMultiplier)))
      (Class|BPISteamable|Interact(Message) _output_get))))

(event Custom|SetVariables
  (params (Player_Ref :type BP%20First%20Person%20Character%20Object%20Reference))
  (bind _spawncomponent (Variables|/Game/Blueprints/BP_FirstPersonCharacter.BP_FirstPersonCharacter_C|GetSpawnComponent Player_Ref))
  (bind _returnvalue (Transformation|GetWorldLocation _spawncomponent))
  (Variables|Default|SetPlayer%20Ref Player_Ref)
  (Variables|Default|SetStart _returnvalue)
  (Variables|Default|SetEnd (+ _returnvalue (* (Math|Vector|GetForwardVector (Variables|/Game/Blueprints/BP_FirstPersonCharacter.BP_FirstPersonCharacter_C|GetCamera Player_Ref)) (Variables|Default|GetDistanceTrace)))))

(event Custom|Reset
  (bind _player_ref (Variables|Default|GetPlayer%20Ref))
  (bind _spawncomponent (Variables|/Game/Blueprints/BP_FirstPersonCharacter.BP_FirstPersonCharacter_C|GetSpawnComponent _player_ref))
  (bind _returnvalue (Transformation|GetWorldLocation _spawncomponent))
  (Variables|Default|SetStart _returnvalue)
  (Variables|Default|SetEnd (+ _returnvalue (* (Math|Vector|GetForwardVector (Variables|/Game/Blueprints/BP_FirstPersonCharacter.BP_FirstPersonCharacter_C|GetCamera _player_ref)) (Variables|Default|GetDistanceTrace)))))

(event EventBeginPlay
  (bind _defaultsceneroot (Variables|Default|GetDefaultSceneRoot))
  (bind _returnvalue (Transformation|GetWorldLocation _defaultsceneroot))
  (|CallParentFunction)
  (Utilities|IsValid (Variables|Default|GetEmitter)
    (:Is%20Valid
      (Audio|PlaySoundatLocation "/Game/Audio/SFX/Environment/Elements/Wind_Start.Wind_Start" _returnvalue "0, 0, 0" 1.0 1.0 0.0 0 0 0 0)
      (bind _returnvalue_2 (Effects|SpawnEmitteratLocation (Variables|Default|GetEmitter) (- _returnvalue "0.000000,0.000000,30.000000") "0, 0, 0" "1.000000,1.000000,1.000000" false))
      (Components|Activation|Deactivate _returnvalue_2))
    (:Is%20Not%20Valid
      (Development|PrintString "Spawn, No emitter"))))

(fn ConstructionScript
  (|CallParentFunction))

(fn ReSetEnd
  (return "0, 0, 0"))

(fn GetDirection
  (return (Math|Vector|GetForwardVector (Transformation|GetWorldRotation (Variables|/Game/Blueprints/BP_FirstPersonCharacter.BP_FirstPersonCharacter_C|GetCamera (Variables|Default|GetPlayer%20Ref))))))