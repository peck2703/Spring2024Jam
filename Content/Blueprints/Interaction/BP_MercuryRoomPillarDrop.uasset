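; Mercury room pillar actor that drops in two stages as part of what appears to be a ball puzzle.
; DropHalfway runs a timeline lerping toward half the difference between current and final locations, recomputed each update rather than a fixed midpoint.
; FallAllWayDown requires CorrectSphereCollider on the first two Ball_Solution actors and a location differing from that halfway value.
; It then lerps from the current location to DesiredFinalLocation on a second timeline.
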(event Custom|DropHalfway
  (bind _returnvalue (Transformation|GetActorLocation))
  (bind _alpha (Timeline|Timeline Play)
    (:Update
      (Transformation|SetActorLocation (Math|Vector|Lerp(Vector) _returnvalue (/ (- _returnvalue (Variables|Default|GetDesiredFinalLocation)) 2.0) _alpha) false false))))

(event Custom|FallAllWayDown
  (bind _returnvalue (Transformation|GetActorLocation))
  (bind _outactors (Actor|GetAllActorsOfClass "/Game/Blueprints/Interaction/Ball_Solution.Ball_Solution_C"))
  (if (Math|Boolean|ANDBoolean (Variables|/Game/Blueprints/Interaction/Ball_Solution.Ball_Solution_C|GetCorrectSphereCollider (Utilities|Array|Get(acopy) _outactors)) (Variables|/Game/Blueprints/Interaction/Ball_Solution.Ball_Solution_C|GetCorrectSphereCollider (Utilities|Array|Get(acopy) _outactors 1)) (Utilities|Operators|NotEqual(!=) _returnvalue (/ (- _returnvalue (Variables|Default|GetDesiredFinalLocation)) 2.0) 0.0))
    (bind _alpha (Timeline|AllWayTimeline Play)
      (:Update
        (Transformation|SetActorLocation (Math|Vector|Lerp(Vector) (Transformation|GetActorLocation) (Variables|Default|GetDesiredFinalLocation) _alpha) false false)))))

(event EventBeginPlay)

(event Collision|EventActorBeginOverlap
  (params (OtherActor :type Actor%20Object%20Reference)))

(event EventTick
  (params (DeltaSeconds :type Float%20%28single-precision%29)))

(fn ConstructionScript)