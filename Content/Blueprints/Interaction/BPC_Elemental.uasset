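; Player component that holds two chosen element classes and combines them into a spawned elemental spell.
; New picks fill open slots or push out the oldest, then refresh the player's element icons.
; CheckElements validates both slots, reduces class display names to short strings by substring match, then switches on the pair through per-element macros.
; Either order yields Steam, Magma, Lightning, Clay, Erosion or Mushroom, some of which also set player state.
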(event Custom|CheckElements
  (if (CallFunction|ValidClassesSelected)
    ;[0 0 0] This will choose the final element that will "Spawn"
    (CallFunction|ChooseSecondaryElement)
    (else
      ;[0 0 0] Must Have two Elements
      (Development|PrintString "Insufficient Elements"))))

(event Custom|FindNextOpenSlot
  (params (Item :type BP%20Element%20M%20Class%20Reference))
  (bind _chosenelement (Variables|Default|GetChosenElement))
  (if (not (Utilities|IsValidClass (Utilities|Array|Get(acopy) _chosenelement)))
    (bind _output_get (Variables|Default|SetEmptyIndex 0))
    (Variables|Default|SetSuccess? true)
    (Utilities|Array|SetArrayElem (Variables|Default|GetChosenElement) _output_get Item true)
    (CallFunction|UpdateIcons)
    (elif (not (Utilities|IsValidClass (Utilities|Array|Get(acopy) _chosenelement 1)))
      (bind _output_get_2 (Variables|Default|SetEmptyIndex 1))
      (Variables|Default|SetSuccess? true)
      (Utilities|Array|SetArrayElem (Variables|Default|GetChosenElement) _output_get_2 Item true)
      (CallFunction|UpdateIcons)
      (else
        (Variables|Default|SetSuccess? false)
        (CallFunction|ChangeSlots Item)
        (CallFunction|UpdateIcons)))))

(event Custom|ChangeSlots
  (params (New%20Element :type BP%20Element%20M%20Class%20Reference%20%28by%20ref%29))
  (bind _chosenelement (Variables|Default|GetChosenElement))
  ;[0 0 0] Move last slot to first
  (Utilities|Array|SetArrayElem _chosenelement 0 (Utilities|Array|Get(acopy) _chosenelement 1))
  ;[0 0 0] Set new power to last slot
  (Utilities|Array|SetArrayElem _chosenelement 1 New%20Element))

(event Custom|RemoveAll
  (Utilities|Array|Clear (Variables|Default|GetChosenElement))
  (Default|CheckElementIcons (Variables|Default|GetPlayer_Ref)))

(fn ValidClassesSelected
  ;[0 0 0] Checks that both slots in the elements list are valid classes
  (bind _array_element (Utilities|Array|ForEachLoopwithBreak (Variables|Default|GetChosenElement) :!label _label)
    (:LoopBody
      (if (not (Utilities|IsValidClass _array_element))
        (goto _label Break)))
    (:Completed
      (return (Utilities|IsValidClass _array_element)))))

(fn ChooseSecondaryElement
  (bind _elementshortnames (Variables|Default|GetElementShortNames))
  (bind _output (Utilities|Array|Get(acopy) _elementshortnames 1))
  (for (_array_element _array_index) (Variables|Default|GetChosenElement)
    ;[0 0 0] Takes the element class' name and shortens for Switch Statements
    (CallFunction|ShortNamingElements _array_element _array_index))
  (switch string (Utilities|Array|Get(acopy) (Variables|Default|GetElementShortNames))
    (:Fire
      (switch string _output
        (:Water
          (|FireFirst :!label _label))
        (:Earth
          (goto _label Magma))
        (:Air
          (goto _label Lightning))))
    (:Water
      (switch string _output
        (:Fire
          (|WaterFirst :!label _label_2))
        (:Earth
          (goto _label_2 Clay))
        (:Air
          (goto _label_2 Erosion))))
    (:Earth
      (switch string _output
        (:Fire
          (|EarthFirst :!label _label_3))
        (:Water
          (goto _label_3 Clay))
        (:Air
          (goto _label_3 Mushroom))))
    (:Air
      (switch string _output
        (:Fire
          (|AirFirst :!label _label_4))
        (:Water
          (goto _label_4 Erosion))
        (:Earth
          (goto _label_4 Mushroom))))))

(fn ShortNamingElements
  (params (Element :type BP%20Element%20M%20Class%20Reference) (Index :type Integer))
  (LocalVariables|SetLocalElement Element)
  (LocalVariables|SetLocalIndex Index)
  (if (Utilities|String|Contains (Utilities|GetClassDisplayName (LocalVariables|GetLocalElement)) "Fire")
    (Utilities|Array|SetArrayElem (Variables|Default|GetElementShortNames) (LocalVariables|GetLocalIndex) "Fire" true)
    (elif (Utilities|String|Contains (Utilities|GetClassDisplayName (LocalVariables|GetLocalElement)) "Water")
      (Utilities|Array|SetArrayElem (Variables|Default|GetElementShortNames) (LocalVariables|GetLocalIndex) "Water" true)
      (elif (Utilities|String|Contains (Utilities|GetClassDisplayName (LocalVariables|GetLocalElement)) "Earth")
        (Utilities|Array|SetArrayElem (Variables|Default|GetElementShortNames) (LocalVariables|GetLocalIndex) "Earth" true)
        (elif (Utilities|String|Contains (Utilities|GetClassDisplayName (LocalVariables|GetLocalElement)) "Air")
          (Utilities|Array|SetArrayElem (Variables|Default|GetElementShortNames) (LocalVariables|GetLocalIndex) "Air" true)
          (return))))))

(fn Steam
  (Game|SpawnActorfromClass "/Game/Blueprints/Interaction/Elements/BP_Element_Steam.BP_Element_Steam_C" (Math|Transform|MakeTransform (Variables|/Game/Blueprints/BP_FirstPersonCharacter.BP_FirstPersonCharacter_C|GetSpawnSpell (Variables|Default|GetPlayer_Ref)) "0, 0, 0" "1.000000,1.000000,1.000000") "Undefined" "MultiplyWithRoot" 0 0 0))

(fn Magma
  (Game|SpawnActorfromClass "/Game/Blueprints/Interaction/Elements/BP_Element_Magma.BP_Element_Magma_C" (Math|Transform|MakeTransform (Variables|/Game/Blueprints/BP_FirstPersonCharacter.BP_FirstPersonCharacter_C|GetSpawnSpell (Variables|Default|GetPlayer_Ref)) "0, 0, 0" "1.000000,1.000000,1.000000") "Undefined" "MultiplyWithRoot" 0 0 0))

(fn Lightning
  (Game|SpawnActorfromClass "/Game/Blueprints/Interaction/Elements/BP_Element_Lightning.BP_Element_Lightning_C" (Math|Transform|MakeTransform (Variables|/Game/Blueprints/BP_FirstPersonCharacter.BP_FirstPersonCharacter_C|GetSpawnSpell (Variables|Default|GetPlayer_Ref)) "0, 0, 0" "1.000000,1.000000,1.000000") "Undefined" "MultiplyWithRoot" 0 0 0))

(fn Erosion
  (bind _player_ref (Variables|Default|GetPlayer_Ref))
  (Development|PrintString "Erosion")
  (bind _returnvalue (Game|SpawnActorfromClass "/Game/Blueprints/Interaction/Elements/BP_Element_Erosion.BP_Element_Erosion_C" (Math|Transform|MakeTransform (CallFunction|PlayerSpawnSpellLocation _player_ref) "0, 0, 0" "1.000000,1.000000,1.000000") "Undefined" "MultiplyWithRoot" 0 _player_ref 0))
  (Default|BeginPower _returnvalue))

(fn Mushroom
  (bind _player_ref (Variables|Default|GetPlayer_Ref))
  (bind _returnvalue (Game|SpawnActorfromClass "/Game/Blueprints/Interaction/Elements/BP_Element_Mushrooms.BP_Element_Mushrooms_C" (Math|Transform|MakeTransform (CallFunction|PlayerSpawnSpellLocation _player_ref) "0, 0, 0" "1.000000,1.000000,1.000000") "Undefined" "MultiplyWithRoot" 0 _player_ref 0))
  (Variables|/Game/Blueprints/BP_FirstPersonCharacter.BP_FirstPersonCharacter_C|SetCurrentMushroom _player_ref _returnvalue)
  (Variables|/Game/Blueprints/BP_FirstPersonCharacter.BP_FirstPersonCharacter_C|SetMushroom _player_ref true))

(fn Clay
  (bind _player_ref (Variables|Default|GetPlayer_Ref))
  (bind _spawncomponent (Variables|/Game/Blueprints/BP_FirstPersonCharacter.BP_FirstPersonCharacter_C|GetSpawnComponent _player_ref))
  (bind _returnvalue (Transformation|GetWorldLocation _spawncomponent))
  (bind _returnvalue_2 (Game|SpawnActorfromClass "/Game/Blueprints/Interaction/Elements/BP_Element_Clay.BP_Element_Clay_C" (Math|Transform|MakeTransform _returnvalue "0, 0, 0" "1.000000,1.000000,1.000000") "Undefined" "MultiplyWithRoot" 0 _returnvalue _player_ref 0))
  (Variables|/Game/Blueprints/BP_FirstPersonCharacter.BP_FirstPersonCharacter_C|SetCurrentClay _player_ref _returnvalue_2)
  (Variables|/Game/Blueprints/BP_FirstPersonCharacter.BP_FirstPersonCharacter_C|SetScroll _player_ref true))

(fn UpdateIcons
  (Default|CheckElementIcons (Variables|Default|GetPlayer_Ref)))

(fn PlayerSpawnSpellLocation
  (params (Player_Ref :type BP%20First%20Person%20Character%20Object%20Reference))
  (return (Transformation|GetWorldLocation (Variables|/Game/Blueprints/BP_FirstPersonCharacter.BP_FirstPersonCharacter_C|GetSpawnComponent Player_Ref))))