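; Lightning rod interactable for Salt Room 2 that changes the room's layout when activated.
; Its Activate event extends a Salt_MovableFloor and then lowers a Salt_StoneDoor_Lower.
; Both targets are found at runtime with GetAllActorsOfClass, using only the first result of each with no validity check.
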(event EventBeginPlay
  (|CallParentFunction) ; This node is disabled and will not be called.\nDrag off pins to build functionality.
)

(event Collision|EventActorBeginOverlap
  (params (OtherActor :type Actor%20Object%20Reference))
  (|CallParentFunction OtherActor) ; This node is disabled and will not be called.\nDrag off pins to build functionality.
)

(event EventTick
  (params (DeltaSeconds :type Float%20%28single-precision%29))
  (|CallParentFunction DeltaSeconds) ; This node is disabled and will not be called.\nDrag off pins to build functionality.
)

(event EventActivate
  (bind _outactors (Actor|GetAllActorsOfClass "/Game/Blueprints/Salt_MovableFloor.Salt_MovableFloor_C"))
  (Default|Extend (Utilities|Array|Get(acopy) _outactors))
  (bind _outactors_2 (Actor|GetAllActorsOfClass "/Game/Blueprints/Salt_StoneDoor_Lower.Salt_StoneDoor_Lower_C"))
  (Default|Lower (Utilities|Array|Get(acopy) _outactors_2)))

(fn ConstructionScript
  (|CallParentFunction))